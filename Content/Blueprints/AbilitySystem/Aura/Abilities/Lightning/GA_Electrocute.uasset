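; GA_Electrocute is a channeled lightning ability that shows a beam cue while input is held.
; It stores cursor target data, faces the target and plays a montage, whose event disables movement and spawns the beam.
; SpawnBeam traces the first target and adds ShockLoop on it if it implements CombatInterface, otherwise on the avatar.
; Input release removes the cue, restores movement and cursor, and ends; CommitAbility is unconnected.
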(event `self.K2_ActivateAbility`
  (if (`KismetSystemLibrary.DoesImplementInterface` (`self.GetAvatarActorFromActorInfo`) "/Script/GAS_RPG.CombatInterface")
    ;[1 1 1] Store Mouse Data Variables
    (bind (_asynctaskproxy _datahandle) (`TargetDataUnderMouse.CreateTargetDataUnderMouse`)
      (:`then`
        (`self.StoreMouseDataInfo` (`AbilitySystemBlueprintLibrary.GetHitResultFromTargetData` _datahandle))
        (`self.StoreOwnerVariables`)
        (`|ExecutionSequence`
          (:`then_0`
            ;[1 1 1] 隐藏鼠标
            (set `PlayerController.bShowMouseCursor` false (`self.OwnerPlayerController`))
            (message `CombatInterface.UpdateFacingTarget` (`self.GetAvatarActorFromActorInfo`) (`self.MouseHitLocation`))
            (`self.K2_ExecuteGameplayCue` (struct :`TagName` "GameplayCue.ShockBurst"))
            (`AbilityTask_PlayMontageAndWait.CreatePlayMontageAndWaitProxy` "None" (`self.Montage_Electrocute`) 1.0 "None" false
              (:`then`
                (`AbilityTask_WaitGameplayEvent.WaitGameplayEvent` (struct :`TagName` "Event.Montage.Electrocute") null true
                  (:`EventReceived`
                    (message `CombatInterface.SetInShockLoop` (`self.GetAvatarActorFromActorInfo`) true)
                    (`CharacterMovementComponent.DisableMovement` (`Character.CharacterMovement` (`self.OwnerCharacter`)))
                    (`self.SpawnBeam`))))))
          (:`then_1`
            (`AbilityTask_WaitInputRelease.WaitInputRelease` false
              (:`OnRelease`
                (set `PlayerController.bShowMouseCursor` true (`self.OwnerPlayerController`))
                (message `CombatInterface.SetInShockLoop` (`self.GetAvatarActorFromActorInfo`) false)
                (`CharacterMovementComponent.SetMovementMode` (`Character.CharacterMovement` (`self.OwnerCharacter`)) "MOVE_Walking" 0)
                (`self.RemoveBeam`)
                (`self.K2_EndAbility`)))))))
    (else
      (`self.K2_EndAbility`))))

(fn `RemoveBeam`
  (if (`self.IsFirstTargetCharacter`)
    (`GameplayCueFunctionLibrary.RemoveGameplayCueOnActor` (`self.MouseHitActor`) (struct :`TagName` "GameplayCue.ShockLoop") (`self.FirstTargetCueParams`))
    (else
      (`GameplayCueFunctionLibrary.RemoveGameplayCueOnActor` (`self.GetAvatarActorFromActorInfo`) (struct :`TagName` "GameplayCue.ShockLoop") (`self.FirstTargetCueParams`)))))

(fn `SpawnBeam`
  (bind _returnvalue (`KismetSystemLibrary.DoesImplementInterface` (`self.MouseHitActor`) "/Script/GAS_RPG.CombatInterface"))
  (`self.TraceFirstTarget` (`self.MouseHitLocation`))
  (bind _returnvalue_2 (message `CombatInterface.GetWeapon` (`self.OwnerCharacter`)))
  (set `self.FirstTargetCueParams` (`AbilitySystemBlueprintLibrary.MakeGameplayCueParameters` 0.0 0.0 (struct) (struct) (struct) (struct) (struct) (`self.MouseHitLocation`) (0.0 0.0 0.0) null null (`self.MouseHitActor`) null 1 1 _returnvalue_2))
  (set `self.IsFirstTargetCharacter` _returnvalue)
  (if _returnvalue
    (set `self.CueTarget` (`self.MouseHitActor`))
    (else
      (set `self.CueTarget` (`self.GetAvatarActorFromActorInfo`))))
  (`GameplayCueFunctionLibrary.AddGameplayCueOnActor` (`self.CueTarget`) (struct :`TagName` "GameplayCue.ShockLoop") (`self.FirstTargetCueParams`)))