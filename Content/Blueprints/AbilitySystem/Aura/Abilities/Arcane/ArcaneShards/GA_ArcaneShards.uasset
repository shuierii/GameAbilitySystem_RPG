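; Arcane Shards gameplay ability that shows a magic circle, then waits for input to target the point under the mouse.
; It turns the avatar toward that point, plays the cast montage, and on its gameplay event spawns a point collection there.
; A looping timer steps through the collection's ground points, firing a shard GameplayCue and debug sphere at each.
; After the last point it destroys the collection and ends the ability.
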(event `self.K2_ActivateAbility`
  (`|ExecutionSequence`
    (:`then_0`
      (message `PlayerInterface.ShowMagicCircle` (`self.GetAvatarActorFromActorInfo`) null))
    (:`then_1`
      (`AbilityTask_WaitInputPress.WaitInputPress` false
        (:`OnPress`
          (bind (_asynctaskproxy _datahandle) (`TargetDataUnderMouse.CreateTargetDataUnderMouse`)
            (:`then`
              (set `self.Impact Point` (`.ImpactPoint` (`GameplayStatics.BreakHitResult` (`AbilitySystemBlueprintLibrary.GetHitResultFromTargetData` _datahandle))))
              (message `CombatInterface.UpdateFacingTarget` (`self.GetAvatarActorFromActorInfo`) (`self.Impact Point`))
              (`AbilityTask_PlayMontageAndWait.CreatePlayMontageAndWaitProxy` "None" "/Game/Assets/Characters/Aura/Animations/Abilities/AM_Cast_ArcaneShards.AM_Cast_ArcaneShards" 1.0 "None" false
                (:`then`
                  (`AbilityTask_WaitGameplayEvent.WaitGameplayEvent` (struct :`TagName` "Event.Montage.ArcaneShards") null true
                    (:`then`
                      (bind _returnvalue (`|SpawnActorFromClass` "/Game/Blueprints/AbilitySystem/Aura/Abilities/Arcane/ArcaneShards/BP_PointCollection.BP_PointCollection_C" (`KismetMathLibrary.MakeTransform` (`self.Impact Point`)) "AlwaysSpawn" "MultiplyWithRoot" null null))
                      (bind _output_get (set `self.PointCollection` _returnvalue))
                      (set `self.GroundPoints` (`PointCollection.GetGroundPoints` _output_get (`self.SpawnLocation`) (`self.Num Points`) 0.0))
                      (bind _returnvalue_2 (`KismetSystemLibrary.K2_SetTimerDelegate` (delegate `SpawnShard`) (`self.Time`) true))
                      (set `self.SpawnTimer` _returnvalue_2)
                      (message `PlayerInterface.HideMagicCircle` (`self.GetAvatarActorFromActorInfo`)))))))))))))

(event `SpawnShard`
  (if (< (`self.Index`) (`self.Num Points`))
    (bind _output_get (set `self.SpawnLocation` (`SceneComponent.K2_GetComponentLocation` (`|GetArrayItem` (`self.GroundPoints`) (`self.Index`)))))
    (`KismetSystemLibrary.DrawDebugSphere` _output_get 20.0 12 (struct :`R` 1.0 :`G` 1.0 :`B` 1.0 :`A` 1.0) 20.0)
    (`/Engine/EditorBlueprintResources/StandardMacros.IncrementInt` (`self.Index`)
      (:`  `
        (`self.K2_ExecuteGameplayCueWithParams` (struct :`TagName` "GameplayCue.ArcaneShard") (`AbilitySystemBlueprintLibrary.MakeGameplayCueParameters` 0.0 0.0 (struct) (struct) (struct) (struct) (struct) (`self.SpawnLocation`)))))
    (else
      (`KismetSystemLibrary.K2_ClearAndInvalidateTimerHandle` (`self.SpawnTimer`))
      (`KismetSystemLibrary.Delay` 0.2)
      (`Actor.K2_DestroyActor` (`self.PointCollection`))
      (`self.K2_EndAbility`))))