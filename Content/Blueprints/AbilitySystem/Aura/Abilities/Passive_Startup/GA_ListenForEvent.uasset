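; A passive gameplay ability that listens for attribute gameplay events on its owner and turns them into a self-applied gameplay effect.
; On activation it waits for any event under the Attributes tag hierarchy, then builds a spec from EventBasedEffectClass.
; The event's tag receives its magnitude via SetByCaller and every other tag in EventTags gets zero before the spec is applied.
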(event `self.K2_ActivateAbility`
  (bind _returnvalue (`self.GetAbilitySystemComponentFromActorInfo`))
  (`KismetSystemLibrary.PrintString` "Hello")
  (bind (_asynctaskproxy _payload) (`AbilityTask_WaitGameplayEvent.WaitGameplayEvent` (struct :`TagName` "Attributes") null false false)
    (:`EventReceived`
      (bind (_eventtag _instigator _target _optionalobject _optionalobject2 _contexthandle _instigatortags _targettags _eventmagnitude) (break `GameplayEventData` _payload))
      (set `self.Event Tag` _eventtag)
      (set `self.Event Magnitude` _eventmagnitude)
      (set `self.Spec` (`AbilitySystemComponent.MakeOutgoingSpec` _returnvalue (`self.EventBasedEffectClass`) 1.0 (`AbilitySystemComponent.MakeEffectContext` _returnvalue)))
      (for _array_element (`self.EventTags`)
        (if (`BlueprintGameplayTagLibrary.MatchesTag` _array_element (`self.Event Tag`) true)
          (`AbilitySystemBlueprintLibrary.AssignTagSetByCallerMagnitude` (`self.Spec`) (`self.Event Tag`) (`self.Event Magnitude`))
          (else
            (`AbilitySystemBlueprintLibrary.AssignTagSetByCallerMagnitude` (`self.Spec`) _array_element))))
      (`AbilitySystemComponent.BP_ApplyGameplayEffectSpecToSelf` (`self.GetAbilitySystemComponentFromActorInfo`) (`self.Spec`)))))