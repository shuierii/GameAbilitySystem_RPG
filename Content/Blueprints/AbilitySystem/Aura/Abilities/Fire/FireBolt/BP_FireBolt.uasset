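; BP_FireBolt is the actor for the Fire Bolt ability, with a fallback that detonates the bolt when it stops moving.
; Each Tick it compares its current location with the previous frame's and treats movement at or below MinDistance as a stop.
; It then plays the impact sound, spawns the Niagara fire explosion at that location and destroys itself, without using overlap or hit events in this graph.
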(event `self.ReceiveTick`
  (params (DeltaSeconds :type "Float (single-precision)"))
  (set `self.LocationLastFram` (`self.LocationThisFram`))
  (set `self.LocationThisFram` (`self.K2_GetActorLocation`))
  (if (<= (`KismetMathLibrary.VSize` (- (`self.LocationThisFram`) (`self.LocationLastFram`))) (`self.MinDistance`))
    (`GameplayStatics.SpawnSoundAtLocation` "/Game/Assets/Sounds/Abilities/FireBolt/sfx_FireBolt_Impact.sfx_FireBolt_Impact" (`self.LocationThisFram`) (struct) 1.0 1.0 0.0 null null)
    (`NiagaraFunctionLibrary.SpawnSystemAtLocation` "/Game/Assets/Effects/Projectiles/FireExplosion/NS_FireExplosion1.NS_FireExplosion1" (`self.LocationThisFram`))
    (`self.K2_DestroyActor`)))

(fn `UserConstructionScript`)