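; GA_FireBolt is the gameplay ability that casts fire bolt projectiles at the target under the mouse.
; After committing, it gets mouse target data, turns the avatar toward the hit location through CombatInterface, and plays the cast montage.
; The montage's gameplay event triggers SpawnProjectiles from the weapon socket with an overridden launch pitch, passing the hit actor as homing target, then ends the ability.
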(event `self.K2_ActivateAbility`
  ;[1 1 1] 检查消耗
  (`self.K2_CommitAbility`)
  (bind (_asynctaskproxy _datahandle) (`TargetDataUnderMouse.CreateTargetDataUnderMouse`)
    (:`then`
      (bind (_bblockinghit _binitialoverlap _time _distance _location _impactpoint _normal _impactnormal _physmat _hitactor) (`GameplayStatics.BreakHitResult` (`AbilitySystemBlueprintLibrary.GetHitResultFromTargetData` _datahandle)))
      (set `self.Location` _location)
      (set `self.Mouse Hit Actor` _hitactor)
      (bind _ascombat_interface (cast `CombatInterface` (`self.GetAvatarActorFromActorInfo`)))
      (`CombatInterface.UpdateFacingTarget` _ascombat_interface (`self.Location`))
      (`AbilityTask_PlayMontageAndWait.CreatePlayMontageAndWaitProxy` "None" "/Game/Assets/Characters/Aura/Animations/Abilities/AM_Cast_FireBolt.AM_Cast_FireBolt"
        (:`then`
          (`AbilityTask_WaitGameplayEvent.WaitGameplayEvent` (struct :`TagName` "Event.Montage.FireBolt") null
            (:`EventReceived`
              (`self.SpawnProjectiles` (`self.Location`) (`BlueprintGameplayTagLibrary.MakeLiteralGameplayTag` (struct :`TagName` "CombatSocket.Weapon")) true 65.0 (`self.Mouse Hit Actor`))
              (`self.K2_EndAbility`))))))))