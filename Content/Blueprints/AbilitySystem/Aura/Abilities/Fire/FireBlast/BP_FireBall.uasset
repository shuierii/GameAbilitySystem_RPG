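; BP_FireBall is the projectile for the Fire Blast ability, flying outward and returning to its ReturnToActor like a boomerang.
; StartOutgoingTimeline runs on authority, using a timeline to lerp from the spawn location to an apex TravelDistance ahead.
; A second timeline lerps back to the actor's live location.
; Within ExplodeDistance of that actor on the return leg, it calls OnHit and destroys itself.
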(event `self.StartOutgoingTimeline`
  (`/Engine/EditorBlueprintResources/ActorMacros.Switch Has Authority`
    (:`Authority`
      (set `self.InitLocation` (`self.K2_GetActorLocation`))
      (set `self.ApexLocation` (+ (`self.InitLocation`) (* (`self.GetActorForwardVector`) (`self.TravelDistance`))))
      (bind (_direction `_新建轨道_0`) (`Timeline|Outgoing`)
        (:`Update`
          (`self.K2_SetActorLocation` (`KismetMathLibrary.VLerp` (`self.InitLocation`) (`self.ApexLocation`) `_新建轨道_0`)))
        (:`Finished`
          (bind (_direction_2 `_新建轨道_0_2`) (`Timeline|Returning`)
            (:`Update`
              (`self.K2_SetActorLocation` (`KismetMathLibrary.VLerp` (`self.ApexLocation`) (`self.K2_GetActorLocation` (`self.ReturnToActor`)) `_新建轨道_0_2`))
              (if (<= (`KismetMathLibrary.VSize` (- (`self.K2_GetActorLocation`) (`self.K2_GetActorLocation` (`self.ReturnToActor`)))) (`self.ExplodeDistance`))
                (`self.OnHit`)
                (`self.K2_DestroyActor`)))))))))

(fn `UserConstructionScript`)