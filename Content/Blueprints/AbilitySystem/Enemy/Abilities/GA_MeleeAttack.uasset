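; Enemy melee attack ability that turns the avatar toward its combat target and plays a random attack montage.
; When the montage's tagged gameplay event arrives, it runs a small sphere query for live players at that montage's combat socket.
; Non-friendly hits take damage, and any hit fires one MeleeImpact gameplay cue carrying the montage tag.
; The ability ends after the hit check or when the montage completes, is interrupted or is cancelled.
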(event `self.K2_ActivateAbility`
  (bind _returnvalue (`self.GetAvatarActorFromActorInfo`))
  (bind _returnvalue_2 (`self.GetAvatarActorFromActorInfo`))
  (bind (_montage _montagetag _sockettag) (break `TaggedMontage` (`self.Tagged Montage`)))
  (set `self.HasHitTarget` false)
  (bind _returnvalue_3 (message `EnemyInterface.GetCombatTarget` (`self.GetAvatarActorFromActorInfo`)))
  (bind _ascombat_interface (cast `CombatInterface` _returnvalue_3))
  (`CombatInterface.UpdateFacingTarget` _ascombat_interface (`Actor.K2_GetActorLocation` _returnvalue_3))
  (bind _returnvalue_4 (message `CombatInterface.GetAttackMontages` (`self.GetAvatarActorFromActorInfo`)))
  (set `self.Tagged Montage` (`self.GetRandomTaggedMontageFromArray` _returnvalue_4))
  (`AbilityTask_PlayMontageAndWait.CreatePlayMontageAndWaitProxy` "None" _montage 1.0 "None" false
    (:`then`
      (`AbilityTask_WaitGameplayEvent.WaitGameplayEvent` _montagetag null
        (:`EventReceived`
          (bind _returnvalue_5 (message `CombatInterface.GetCombatSocketLocation` _returnvalue _sockettag))
          (bind _output_get (set `self.CombatSocketLocation` _returnvalue_5))
          (bind _outoverlappingactors (`AuraAbilitySystemLibrary.GetLivePlayersWithinRadius` _returnvalue (`|MakeArray` _returnvalue) 45.0 _output_get))
          (for _array_element _outoverlappingactors
            (bind _returnvalue_6 (`AuraAbilitySystemLibrary.IsNotFriend` (`self.GetAvatarActorFromActorInfo`) _array_element))
            (if _returnvalue_6
              (`self.CauseDamage` _array_element)
              (set `self.HasHitTarget` true)))
          (if (`self.HasHitTarget`)
            (bind _returnvalue_7 (message `EnemyInterface.GetCombatTarget` _returnvalue_2))
            (`self.K2_ExecuteGameplayCueWithParams` (struct :`TagName` "GameplayCue.MeleeImpact") (`AbilitySystemBlueprintLibrary.MakeGameplayCueParameters` 0.0 0.0 (struct) (struct) (struct) (`BlueprintGameplayTagLibrary.MakeGameplayTagContainerFromTag` (`.MontageTag` (break `TaggedMontage` (`self.Tagged Montage`)))) (struct) (`self.CombatSocketLocation`) (0.0 0.0 0.0) null _returnvalue_2 _returnvalue_7)))
          (`self.K2_EndAbility`))))
    (:`OnCompleted`
      (`self.K2_EndAbility` :!label _label))
    (:`OnInterrupted`
      (goto _label))
    (:`OnCancelled`
      (goto _label))))