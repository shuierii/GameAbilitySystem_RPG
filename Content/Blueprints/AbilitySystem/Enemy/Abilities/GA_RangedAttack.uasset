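; Enemy ranged attack gameplay ability that fires a projectile at the avatar's current combat target.
; On activation it turns toward the target through CombatInterface and plays a random tagged attack montage.
; A gameplay event matching a montage tag triggers SpawnProjectile from a tagged socket toward the target's location at that moment.
; The ability ends when the montage completes, is interrupted or is cancelled.
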(event `self.K2_ActivateAbility`
  (bind _returnvalue (message `EnemyInterface.GetCombatTarget` (`self.GetAvatarActorFromActorInfo`)))
  (bind _ascombat_interface (cast `CombatInterface` _returnvalue))
  (`CombatInterface.UpdateFacingTarget` _ascombat_interface (`Actor.K2_GetActorLocation` _returnvalue))
  (bind _returnvalue_2 (message `CombatInterface.GetAttackMontages` (`self.GetAvatarActorFromActorInfo`)))
  (bind (_montage _montagetag _sockettag) (break `TaggedMontage` (`self.GetRandomTaggedMontageFromArray` _returnvalue_2)))
  (`AbilityTask_PlayMontageAndWait.CreatePlayMontageAndWaitProxy` "None" _montage 1.0 "None" false
    (:`then`
      (`AbilityTask_WaitGameplayEvent.WaitGameplayEvent` _montagetag null
        (:`EventReceived`
          (bind _returnvalue_3 (message `EnemyInterface.GetCombatTarget` (`self.GetAvatarActorFromActorInfo`)))
          (`self.SpawnProjectile` (`Actor.K2_GetActorLocation` _returnvalue_3) _sockettag))))
    (:`OnCompleted`
      (`self.K2_EndAbility` :!label _label))
    (:`OnInterrupted`
      (goto _label))
    (:`OnCancelled`
      (goto _label))))