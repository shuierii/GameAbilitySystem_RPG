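; Base pickup actor that bounces when it spawns, then switches to sine-driven movement and rotation.
; A BeginPlay timeline offsets Z from the initial location, scaled by SpawnApex, then calls StartSinMovement and StartSinRotation, which are defined outside these graphs.
; Tick applies the calculated location and rotation without sweeping.
; Sounds play on spawn, once when the bounce curve dips below its start, and on destruction as the consume cue.
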(event `self.ReceiveBeginPlay`
  (`GameplayStatics.SpawnSoundAtLocation` (`self.SpawnSound`) (`self.K2_GetActorLocation`) (struct) 1.0 1.0 0.0 null null)
  (bind (_direction `_新建轨道_0`) (`Timeline|时间轴`)
    (:`Update`
      ;[1 1 1] 弹跳一下
      (set `self.CalculatedLocation` (`KismetMathLibrary.MakeVector` (.x (`self.InitialLocation`)) (.y (`self.InitialLocation`)) (+ (.z (`self.InitialLocation`)) (* `_新建轨道_0` (`self.SpawnApex`)))))
      (if (< `_新建轨道_0` -0.1)
        (`/Engine/EditorBlueprintResources/StandardMacros.DoOnce` false
          (:`Completed`
            (`GameplayStatics.PlaySoundAtLocation` (`self.GroundImpactSound`) (`self.K2_GetActorLocation`) (struct) 1.0 1.0 0.0 null null null null)))))
    (:`Finished`
      (`self.StartSinMovement`)
      (`self.StartSinRotation`))))

(event `self.ReceiveTick`
  (params (DeltaSeconds :type "Float (single-precision)"))
  (`self.K2_SetActorLocation` (`self.CalculatedLocation`))
  (`self.K2_SetActorRotation` (`self.CalculatedRotation`)))

(event `self.ReceiveDestroyed`
  (`GameplayStatics.SpawnSoundAtLocation` (`self.ConsumSound`) (`self.K2_GetActorLocation`) (struct) 1.0 1.0 0.0 null null))

(fn `UserConstructionScript`)