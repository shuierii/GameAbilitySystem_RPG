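; BP_FlamePillar is a flame pillar actor whose point light varies in intensity continuously from BeginPlay, as a flame flicker.
; A random pick plays one of two timelines, and each one picks again on finishing, forming an endless, irregular loop.
; Each timeline update feeds its track value to ScaleFlameIntensity, which multiplies it by BaseIntensity to set the PointLight intensity.
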(event `自定义事件_1`
  (switch `int` (`KismetMathLibrary.RandomIntegerInRange` 0 1)
    (:`Default`
      (`self.自定义事件_0` :!label _label))
    (:`0`
      (`self.自定义事件`))
    (:`1`
      (goto _label))))

(event `自定义事件`
  (bind (_direction `_新建轨道_0`) (`Timeline|时间轴`)
    (:`Update`
      (`self.ScaleFlameIntensity` `_新建轨道_0`))
    (:`Finished`
      (`self.自定义事件_1`))))

(event `self.ReceiveBeginPlay`
  (`self.自定义事件_1`))

(event `自定义事件_0`
  (bind (_direction `_新建轨道_0`) (`Timeline|时间轴_0`)
    (:`Update`
      (`self.ScaleFlameIntensity` `_新建轨道_0`))
    (:`Finished`
      (`self.自定义事件_1`))))

(fn `ScaleFlameIntensity`
  (params (A :type "Float (double-precision)"))
  (`LightComponent.SetIntensity` (`self.PointLight`) (* A (`self.BaseIntensity`))))

(fn `UserConstructionScript`)