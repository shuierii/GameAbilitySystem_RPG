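; BP_Aura_MainMenu is the main menu scene actor, handling menu setup and animating a fire effect and decal.
; On BeginPlay it plays menu music, adds WBP_MainMenu to the viewport, and switches to UI-only input with a visible cursor.
; Each Tick it bobs Fire vertically around its starting location with a sine of a wrapping time counter, and rotates the decal at a configurable rate.
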(event `self.ReceiveBeginPlay`
  (bind _returnvalue (`GameplayStatics.GetPlayerController` 0))
  (set `self.WorldLocation` (`SceneComponent.K2_GetComponentLocation` (`self.Fire`)))
  (`GameplayStatics.PlaySound2D` "/Game/Assets/Sounds/Music/Music_MainMenu.Music_MainMenu" 1.0 1.0 0.0 null null)
  (bind _returnvalue_2 (`|CreateWidget` "/Game/Blueprints/UI/MainMenu/WBP_MainMenu.WBP_MainMenu_C"))
  (`UserWidget.AddToViewport` _returnvalue_2 0)
  (`WidgetBlueprintLibrary.SetInputMode_UIOnlyEx` _returnvalue null)
  (set `PlayerController.bShowMouseCursor` true _returnvalue))

(event `self.ReceiveTick`
  (params (DeltaSeconds :type "Float (single-precision)"))
  (`self.UpdateTime` DeltaSeconds)
  ;[1 1 1] 实现火球上下动态表现
  (`SceneComponent.K2_SetWorldLocation` (`self.Fire`) (+ (`self.WorldLocation`) (`KismetMathLibrary.MakeVector` 0.0 0.0 (* (`KismetMathLibrary.Sin` (`self.Time`)) (`self.Co`)))) false false)
  (`SceneComponent.K2_AddLocalRotation` (`self.Decal`) (`KismetMathLibrary.MakeRotator` (* (`GameplayStatics.GetWorldDeltaSeconds`) (`self.CircleRotaionRate`))) false false))

(fn `UpdateTime`
  (params (B :type "Float (double-precision)"))
  (bind _output_get (set `self.Time` (+ (`self.Time`) B)))
  (if (> _output_get 6.28)
    (set `self.Time` 0.0)))

(fn `UserConstructionScript`)